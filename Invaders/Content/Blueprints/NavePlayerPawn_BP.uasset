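; NavePlayerPawn_BP is a player pawn for a ship ("Nave") that moves along the X and Z axes under gravity.
; Right, left, up and down input presses overwrite the X or Z component of a Movement vector with per-direction speeds and print a debug "Hello".
; Each Tick subtracts delta-scaled Gravity from Z, then applies Movement as an unswept world offset that is not scaled by frame time.
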(event EventBeginPlay)

(event Collision|EventActorBeginOverlap
  (params (OtherActor :type Actor%20Object%20Reference)))

(event EventTick
  (params (DeltaSeconds :type Float%20%28single-precision%29))
  (bind _output_get (Variables|Default|SetMovement (Math|Vector|MakeVector (.x (Variables|Default|GetMovement)) (.y (Variables|Default|GetMovement)) (- (.z (Variables|Default|GetMovement)) (* DeltaSeconds (Variables|Default|GetGravity))))))
  (Transformation|AddActorWorldOffset _output_get))

(event Input|ActionEvents|InputActionNaveDown
  (params (Key :type Key%20Structure))
  (:Pressed
    (Variables|Default|SetMovement (Math|Vector|MakeVector (.x (Variables|Default|GetMovement)) (.y (Variables|Default|GetMovement)) (Variables|Default|GetNaveSpeedDown)))
    (Development|PrintString "Hello")))

(event Input|ActionEvents|InputActionNaveL
  (params (Key :type Key%20Structure))
  (:Pressed
    (Variables|Default|SetMovement (Math|Vector|MakeVector (Variables|Default|GetNaveSpeedL) (.y (Variables|Default|GetMovement)) (.z (Variables|Default|GetMovement))))
    (Development|PrintString "Hello")))

(event Input|ActionEvents|InputActionNaveR
  (params (Key :type Key%20Structure))
  (:Pressed
    (Variables|Default|SetMovement (Math|Vector|MakeVector (Variables|Default|GetNaveSpeedR) (.y (Variables|Default|GetMovement)) (.z (Variables|Default|GetMovement))))
    (Development|PrintString "Hello")))

(event Input|ActionEvents|InputActionNaveUP
  (params (Key :type Key%20Structure))
  (:Pressed
    (Variables|Default|SetMovement (Math|Vector|MakeVector (.x (Variables|Default|GetMovement)) (.y (Variables|Default|GetMovement)) (Variables|Default|GetNaveSpeedUP)))
    (Development|PrintString "Hello")))

(fn ConstructionScript)